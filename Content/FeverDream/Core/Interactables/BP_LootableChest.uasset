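; BP_LootableChest is an interactable loot chest with a base and a lid.
; Its Interact event calls the parent implementation and prints a debug message, with no loot logic in this graph.
; Disconnected leftover logic, which never runs, would rotate the lid through an AnimateLid timeline and play a one-time sound at the base, plus an extra cue when Ethereal is set.
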(event `FDGameplayInterface.Interact`
  (params (InstigatorPawn :type "Pawn Object Reference"))
  (`parent.Interact` null)
  (`KismetSystemLibrary.PrintString` "BP_LootableChest : Interact" true true (struct :`G` 0.66 :`B` 1.0 :`A` 1.0) 10.0))

(fn `UserConstructionScript`)