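; Player controller for FeverDream that sets up the local player's HUD and offers a keyboard shortcut for saving the world.
; On BeginPlay, only for a local controller, it creates the Main_HUD widget, adds it to the viewport and switches input to game only.
; A hardcoded L key press casts the game mode to FDGameModeBase, calls WriteSaveGame and prints a confirmation string.
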(event `self.ReceiveBeginPlay`
  (if (`self.IsLocalController`)
    (bind _returnvalue (`|CreateWidget` "/Game/FeverDream/Core/UI/Main_HUD.Main_HUD_C"))
    (`UserWidget.AddToViewport` _returnvalue 0)
    (`WidgetBlueprintLibrary.SetInputMode_GameOnly` self)))

(event `Key|L`
  (params (Key :type "Key Structure"))
  (:`Pressed`
    (bind _asfdgame_mode_base (cast `FDGameModeBase` (`GameplayStatics.GetGameMode`)))
    (`FDGameModeBase.WriteSaveGame` _asfdgame_mode_base)
    (`KismetSystemLibrary.PrintString` "world save")))

(fn `UserConstructionScript`)