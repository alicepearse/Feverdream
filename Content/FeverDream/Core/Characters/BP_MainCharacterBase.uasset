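; BP_MainCharacterBase is a main character Blueprint that wires parry input and shows health debug output.
; The Parry input starts the "Parry" action by name on ActionComp, with the character as instigator.
; AttributeComp supplies health, which is printed to screen every tick and again in green whenever OnHealthChanged fires.
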(event `self.ReceiveBeginPlay`)

(event `self.ReceiveTick`
  (params (DeltaSeconds :type "Float (single-precision)"))
  (`KismetSystemLibrary.PrintString` (`KismetStringLibrary.Conv_DoubleToString` (`FDAttributeComponent.Health` (`self.AttributeComp`))) true false (struct :`G` 0.66 :`B` 1.0 :`A` 1.0) 0.0))

(event `self.AttributeComp.OnHealthChanged`
  (params (InstigatorActor :type "Actor Object Reference") (OwningComp :type "FDAttributeComponent Object Reference") (NewHealth :type "Float (single-precision)") (NewMaxHealth :type "Float (single-precision)") (Delta :type "Float (single-precision)"))
  (`KismetSystemLibrary.PrintString` (`KismetStringLibrary.Conv_DoubleToString` NewHealth) true true (struct :`R` 0.204079 :`G` 1.0 :`B` 0.207481 :`A` 1.0)))

(event `InputAction|Parry`
  (params (Key :type "Key Structure"))
  (:`Pressed`
    (`FDActionComponent.StartActionByName` (`self.ActionComp`) self "Parry")))

(fn `UserConstructionScript`)